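; BP_PowerUp1 is a spinning pickup that raises an overlapping Character's max walk speed, then destroys itself.
; Tick yaws or pitches the actor in local space and plays a timeline that applies local offsets for movement.
; Any overlap spawns an explosion emitter before the Character cast, and the speed change is never reverted here.
; A separate hit handler destroys the pickup on ThirdPersonCharacter contact without granting the boost.
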(event `self.PowerUp1.OnComponentHit`
  (params (HitComponent :type "PrimitiveComponent Object Reference") (OtherActor :type "Actor Object Reference") (OtherComp :type "PrimitiveComponent Object Reference") (NormalImpulse :type "Vector Structure") (Hit :type "HitResult Structure (by ref)"))
  ;[1 1 1] When the player hits the PowerUp1, they get (XXX)
  (cast `/Game/ThirdPersonCPP/Blueprints/ThirdPersonCharacter` OtherActor)
  (`self.K2_DestroyActor`))

(event `self.ReceiveTick`
  (params (DeltaSeconds :type "Float (single-precision)"))
  (`self.K2_AddActorLocalRotation` (struct :`Pitch` 1.0))
  (bind (_direction _movement) (`Timeline|Blueprint`)
    (:`Update`
      (`self.K2_AddActorLocalOffset` _movement))))

(event `self.PowerUp1.OnComponentBeginOverlap`
  (params (OverlappedComponent :type "PrimitiveComponent Object Reference") (OtherActor :type "Actor Object Reference") (OtherComp :type "PrimitiveComponent Object Reference") (OtherBodyIndex :type Integer) (bFromSweep :type Boolean) (SweepResult :type "HitResult Structure (by ref)"))
  (`GameplayStatics.SpawnEmitterAtLocation` "/Game/StarterContent/Particles/P_Explosion.P_Explosion" (`self.K2_GetActorLocation`))
  (bind _ascharacter (cast `Character` OtherActor))
  (set `CharacterMovementComponent.MaxWalkSpeed` 3000.0 (`Character.CharacterMovement` _ascharacter))
  (`self.K2_DestroyActor`))

(fn `UserConstructionScript`)