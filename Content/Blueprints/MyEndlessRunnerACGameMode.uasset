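; Game mode for an endless runner that shows the run HUD and builds the floor track from tile actors.
; On BeginPlay it creates the HUD widget and lays an opening run of straight tiles.
; Separate add functions spawn default, straight, blocker, permanent blocker, collectable and ramp up/down tiles at NextSpawnPoint.
; Each then stores the new tile's end transform as NextSpawnPoint, chaining tiles end to end.
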(event `self.ReceiveBeginPlay`
  ;[1 1 1] Displays HUD
  (bind _returnvalue (`|CreateWidget` "/Game/Blueprints/BP_RunHUD.BP_RunHUD_C"))
  (`UserWidget.AddToViewport` _returnvalue 0)
  ;[1 1 1] Every 10 tiles, this adds a new tile.
  (for _ (range 7)
    (`self.AddStraightTile`)))

(fn `AddBlockerTile`
  ;[1 1 1] Adds 1 Blocker floor tile, then sets the end of that tile to be the new beginning for a new tile...
  (bind _returnvalue (`|SpawnActorFromClass` "/Game/Blueprints/BP_BlockerTile.BP_BlockerTile_C" (`self.NextSpawnPoint`) "Undefined" "OverrideRootScale" null null))
  (bind _asbp_blocker_tile (cast `/Game/Blueprints/BP_BlockerTile` _returnvalue))
  (bind _tileendtransform (`/Game/Blueprints/BP_DefaultTile.GetTileEndTransform` _asbp_blocker_tile))
  (set `self.NextSpawnPoint` _tileendtransform))

(fn `AddBlockerTilePERMANENT`
  ;[1 1 1] Adds 1 PERMANENT Blocker tile, then sets the end of that tile to be the new beginning for a new tile...
  (bind _returnvalue (`|SpawnActorFromClass` "/Game/Blueprints/BP_BlockerTilePERMANENT.BP_BlockerTilePERMANENT_C" (`self.NextSpawnPoint`) "Undefined" "OverrideRootScale" null null))
  (bind _asbp_blocker_tile_permanent (cast `/Game/Blueprints/BP_BlockerTilePERMANENT` _returnvalue))
  (bind _tileendtransform (`/Game/Blueprints/BP_DefaultTile.GetTileEndTransform` _asbp_blocker_tile_permanent))
  (set `self.NextSpawnPoint` _tileendtransform))

(fn `AddCollectableTile`
  ;[1 1 1] Adds 1 Straight floor tile, then sets the end of that tile to be the new beginning for a new tile...
  (bind _returnvalue (`|SpawnActorFromClass` "/Game/Blueprints/BP_CollectableTile.BP_CollectableTile_C" (`self.NextSpawnPoint`) "Undefined" "OverrideRootScale" null null))
  (bind _asbp_collectable_tile (cast `/Game/Blueprints/BP_CollectableTile` _returnvalue))
  (bind _tileendtransform (`/Game/Blueprints/BP_DefaultTile.GetTileEndTransform` _asbp_collectable_tile))
  (set `self.NextSpawnPoint` _tileendtransform))

(fn `AddDefaultTile`
  ;[1 1 1] Adds 1 Default floor tile, then sets the end of that tile to be the new beginning for a new tile...
  (bind _returnvalue (`|SpawnActorFromClass` "/Game/Blueprints/BP_DefaultTile.BP_DefaultTile_C" (`self.NextSpawnPoint`) "Undefined" "OverrideRootScale" null null))
  (bind _asbp_default_tile (cast `/Game/Blueprints/BP_DefaultTile` _returnvalue))
  (bind _tileendtransform (`/Game/Blueprints/BP_DefaultTile.GetTileEndTransform` _asbp_default_tile))
  (set `self.NextSpawnPoint` _tileendtransform))

(fn `AddRampDownTile`
  ;[1 1 1] Adds 1 Straight floor tile, then sets the end of that tile to be the new beginning for a new tile...
  (bind _returnvalue (`|SpawnActorFromClass` "/Game/Blueprints/BP_DownTile.BP_DownTile_C" (`self.NextSpawnPoint`) "Undefined" "OverrideRootScale" null null))
  (bind _asbp_down_tile (cast `/Game/Blueprints/BP_DownTile` _returnvalue))
  (bind _tileendtransform (`/Game/Blueprints/BP_DefaultTile.GetTileEndTransform` _asbp_down_tile))
  (set `self.NextSpawnPoint` _tileendtransform))

(fn `AddRampUpTile`
  ;[1 1 1] Adds 1 Straight floor tile, then sets the end of that tile to be the new beginning for a new tile...
  (bind _returnvalue (`|SpawnActorFromClass` "/Game/Blueprints/BP_UpTile.BP_UpTile_C" (`self.NextSpawnPoint`) "Undefined" "OverrideRootScale" null null))
  (bind _asbp_up_tile (cast `/Game/Blueprints/BP_UpTile` _returnvalue))
  (bind _tileendtransform (`/Game/Blueprints/BP_DefaultTile.GetTileEndTransform` _asbp_up_tile))
  (set `self.NextSpawnPoint` _tileendtransform))

(fn `AddStraightTile`
  ;[1 1 1] Adds 1 Straight floor tile, then sets the end of that tile to be the new beginning for a new tile...
  (bind _returnvalue (`|SpawnActorFromClass` "/Game/Blueprints/BP_StraightTile.BP_StraightTile_C" (`self.NextSpawnPoint`) "Undefined" "OverrideRootScale" null null))
  (bind _asbp_straight_tile (cast `/Game/Blueprints/BP_StraightTile` _returnvalue))
  (bind _tileendtransform (`/Game/Blueprints/BP_DefaultTile.GetTileEndTransform` _asbp_straight_tile))
  (set `self.NextSpawnPoint` _tileendtransform))

(fn `UserConstructionScript`)