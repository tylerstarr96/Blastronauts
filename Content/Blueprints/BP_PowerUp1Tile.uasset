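; BP_PowerUp1Tile is a tile Blueprint that can place a child actor, named as a blocker, at one of three spawn points.
; SetBlockerSpawnPoints gathers the relative transforms of BlockerSpawn, BlockerSpawnL and BlockerSpawnR into an array.
; SpawnBlocker adds a child actor component at a random entry from that array.
; The event graph and construction script are empty, so neither function is called within this graph.
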(fn `SetBlockerSpawnPoints`
  ;[1 1 1] Takes the locations of all 3 spawners, and converts them into 1 arry/list. Returns the array of locations.
  (set `self.Blocker Spawn Points` (`|MakeArray` (`SceneComponent.GetRelativeTransform` (`self.BlockerSpawn`)) (`SceneComponent.GetRelativeTransform` (`self.BlockerSpawn_L`)) (`SceneComponent.GetRelativeTransform` (`self.BlockerSpawn_R`)))))

(fn `SpawnBlocker`
  (bind _blocker_spawn_points (`self.Blocker Spawn Points`))
  (`AddComponent|NODE_AddChildActorComponent-0` :`RelativeTransform` (`|GetArrayItem` _blocker_spawn_points (`KismetMathLibrary.RandomIntegerInRange` 0 (`KismetArrayLibrary.Array_LastIndex` _blocker_spawn_points)))))

(fn `UserConstructionScript`)