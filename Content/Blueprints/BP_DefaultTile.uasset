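; BP_DefaultTile is a floor tile in an endless runner that extends the track as the player runs over it.
; When a ThirdPersonCharacter overlaps EndTrigger, a random roll picks which tile type the game mode adds next, with unmatched rolls adding another default tile.
; The tile destroys itself after a short delay.
; GetTileEndTransform exposes the world transform of the TileEnd arrow.
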(event `self.EndTrigger.OnComponentBeginOverlap`
  (params (OverlappedComponent :type "PrimitiveComponent Object Reference") (OtherActor :type "Actor Object Reference") (OtherComp :type "PrimitiveComponent Object Reference") (OtherBodyIndex :type Integer) (bFromSweep :type Boolean) (SweepResult :type "HitResult Structure (by ref)"))
  ;[1 1 1] When the player overlaps with the end trigger, spawn a new tile, wait 2 seconds, then destroy itself.
  ;;[1 1 1] Prereq's for spawning in tiles
  (cast `/Game/ThirdPersonCPP/Blueprints/ThirdPersonCharacter` OtherActor)
  (bind _asmy_endless_runner_acgame_mode (cast `/Game/Blueprints/MyEndlessRunnerACGameMode` (`GameplayStatics.GetGameMode`)))
  ;;[1 1 1] Spawning Tiles
  ;;;[-1.945 1 1] Output determines which tile will spawn next...
  (switch `int` (`KismetMathLibrary.RandomIntegerInRange` 0 10)
    (:`Default`
      (`/Game/Blueprints/MyEndlessRunnerACGameMode.AddDefaultTile` _asmy_endless_runner_acgame_mode))
    (:`0`
      (`/Game/Blueprints/MyEndlessRunnerACGameMode.AddStraightTile` _asmy_endless_runner_acgame_mode))
    (:`1`
      (`/Game/Blueprints/MyEndlessRunnerACGameMode.AddBlockerTile` _asmy_endless_runner_acgame_mode))
    (:`2`
      (`/Game/Blueprints/MyEndlessRunnerACGameMode.AddCollectableTile` _asmy_endless_runner_acgame_mode))
    (:`3`
      (`/Game/Blueprints/MyEndlessRunnerACGameMode.AddRampDownTile` _asmy_endless_runner_acgame_mode))
    (:`4`
      (`/Game/Blueprints/MyEndlessRunnerACGameMode.AddRampUpTile` _asmy_endless_runner_acgame_mode))
    (:`5`
      (`/Game/Blueprints/MyEndlessRunnerACGameMode.AddBlockerTilePERMANENT` _asmy_endless_runner_acgame_mode))
    (:`6`
      (`/Game/Blueprints/MyEndlessRunnerACGameMode.AddBarrierTile` _asmy_endless_runner_acgame_mode))
    (:`7`
      (`/Game/Blueprints/MyEndlessRunnerACGameMode.AddPowerUp1Tile` _asmy_endless_runner_acgame_mode)))
  ;;[1 1 1] Postreq's for spawning in tiles
  (`KismetSystemLibrary.Delay` 2.0)
  (`self.K2_DestroyActor`))

(fn `GetTileEndTransform`
  (returns (TileEndTransform :type "Transform Structure"))
  ;[1 1 1] Takes in the arrow and returns the arrow's location
  (return (`SceneComponent.K2_GetComponentToWorld` (`self.TileEnd`))))

(fn `UserConstructionScript`)